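; BP_DiedZone is a kill zone that resets the player and parts of the level on contact.
; A Cube hit from the Player resets the character to Respawm1, stops the Enemy's SliceCreator and resets every ResetObj entry.
; If a Treasure was valid at BeginPlay, it spawns a hinted BP_Treasure at the saved transform.
; SliceAble actors are destroyed, with sliced cones also decrementing BP_R's ConeCnt.
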(event OnComponentHit(Cube)
  (params (HitComponent :type Primitive%20Component%20Object%20Reference) (OtherActor :type Actor%20Object%20Reference) (OtherComp :type Primitive%20Component%20Object%20Reference) (NormalImpulse :type Vector :default "0, 0, 0") (Hit :type Hit%20Result%20Structure%20%28by%20ref%29))
  (bind _enemy (Variables|Default|GetEnemy))
  (if (Actor|ActorHasTag OtherActor "Player")
    (bind _asbp_third_person_character (Utilities|Casting|CastToBP_ThirdPersonCharacter OtherActor))
    (Default|Reset _asbp_third_person_character (Variables|Default|GetRespawm1))
    (Utilities|FlowControl|Sequence
      (:then_0
        (Utilities|IsValid _enemy
          (:Is%20Valid
            (Variables|/Game/BP/BP_SliceCreator.BP_SliceCreator_C|SetWork (Variables|/Game/Variant_Combat/Blueprints/AI/BP_CombatEnemy.BP_CombatEnemy_C|GetSliceCreator _enemy) false))))
      (:then_1
        (for _array_element (Variables|Default|GetResetObj)
          (Default|Reset _array_element))
        (if (Variables|Default|GetCanResetTreasure)
          (bind _returnvalue (Game|SpawnActorfromClass "/Game/BP/BP_Treasure.BP_Treasure_C" (Variables|Default|GetTreasureTrans) "Undefined" "MultiplyWithRoot" 0 0))
          (Variables|/Game/BP/BP_Treasure.BP_Treasure_C|SetHint _returnvalue true)
          (Variables|/Game/BP/BP_Treasure.BP_Treasure_C|SetHintBP _returnvalue "/Game/BP/BP_HintTreasure.BP_HintTreasure_C"))))
    (elif (Actor|ActorHasTag OtherActor "SliceAble")
      (Utilities|Casting|CastToBP_SliceCone OtherActor
        (:then
          (bind _returnvalue_2 (Actor|GetActorOfClass "/Game/BP/BP_R.BP_R_C"))
          (Variables|/Game/BP/BP_R.BP_R_C|SetConeCnt _returnvalue_2 (- (Variables|/Game/BP/BP_R.BP_R_C|GetConeCnt _returnvalue_2) 1)))
        (:CastFailed
          _))
      (Actor|DestroyActor OtherActor))))

(event EventBeginPlay
  (bind _treasure (Variables|Default|GetTreasure))
  (Utilities|IsValid _treasure
    (:Is%20Valid
      (Variables|Default|SetTreasureTrans (Transformation|GetActorTransform _treasure))
      (Variables|Default|SetCanResetTreasure true))))

(event Collision|EventActorBeginOverlap
  (params (OtherActor :type Actor%20Object%20Reference)))

(fn ConstructionScript)