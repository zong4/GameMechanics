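; BP_Treasure is a trigger actor that the player touches to show a hint, travel to a level, or spring an encounter, depending on its flags.
; For two named levels, it unlocks grapple or slice in BP_Instance and saves the player's position before loading.
; On BeginPlay, it destroys itself if that ability is already unlocked.
; The CloseBack branch reveals a blocking cube and activates the Enemy's SliceCreator.
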(event OnComponentBeginOverlap(Cube)
  (params (OverlappedComponent :type Primitive%20Component%20Object%20Reference) (OtherActor :type Actor%20Object%20Reference) (OtherComp :type Primitive%20Component%20Object%20Reference) (OtherBodyIndex :type Integer) (bFromSweep :type Boolean) (SweepResult :type Hit%20Result%20Structure%20%28by%20ref%29))
  (bind _returnvalue (Game|GetPlayerController 0))
  (bind _levelname (Variables|Default|GetLevelName))
  (bind _cube1 (Variables|Default|GetCube1))
  (bind _levelname_2 (Variables|Default|GetLevelName))
  (bind _returnvalue_2 (Pawn|GetControlledPawn _returnvalue))
  (bind _returnvalue_3 (Transformation|GetActorLocation _returnvalue_2))
  (if (Actor|ActorHasTag OtherActor "Player")
    (Components|DestroyComponent (Variables|Default|GetCube))
    (if (Variables|Default|GetHint)
      (bind _returnvalue_4 (UserInterface|CreateWidget (Variables|Default|GetHintBP)))
      (UserInterface|Viewport|AddtoViewport _returnvalue_4 0)
      (Utilities|FlowControl|Delay 1.5)
      (Widget|RemovefromParent _returnvalue_4)
      (Actor|DestroyActor)
      (elif (Variables|Default|GetOpenLevel)
        (if (Utilities|Enum|Equal(Enum) _levelname "Lvl_ThirdPerson")
          (bind _asbp_instance (Utilities|Casting|CastToBP_Instance (Game|GetGameInstance)))
          (if (not (Variables|/Game/ThirdPerson/Blueprints/BP_Instance.BP_Instance_C|GetCanGrap _asbp_instance))
            (Variables|/Game/ThirdPerson/Blueprints/BP_Instance.BP_Instance_C|SetCanGrap _asbp_instance true)
            (Variables|/Game/ThirdPerson/Blueprints/BP_Instance.BP_Instance_C|SetNewPos _asbp_instance true)
            (Variables|/Game/ThirdPerson/Blueprints/BP_Instance.BP_Instance_C|SetPos _asbp_instance _returnvalue_3)
            (Game|OpenLevel(byName) (Utilities|String|StringToName _levelname_2) :!label _label)
            (Actor|DestroyActor)
            (if (Utilities|Enum|NotEqual(Enum) _levelname_2 "World")
              (bind _returnvalue_5 (UserInterface|CreateWidget "/Game/BP/BP_Temple.BP_Temple_C"))
              (UserInterface|Viewport|AddtoViewport _returnvalue_5 0)
              (Utilities|FlowControl|Delay 1.5)
              (Widget|RemovefromParent _returnvalue_5)))
          (elif (Utilities|Enum|Equal(Enum) _levelname "Lv2")
            (bind _asbp_instance_2 (Utilities|Casting|CastToBP_Instance (Game|GetGameInstance)))
            (if (not (Variables|/Game/ThirdPerson/Blueprints/BP_Instance.BP_Instance_C|GetCanSlice _asbp_instance_2))
              (Variables|/Game/ThirdPerson/Blueprints/BP_Instance.BP_Instance_C|SetCanSlice _asbp_instance_2 true)
              (Variables|/Game/ThirdPerson/Blueprints/BP_Instance.BP_Instance_C|SetNewPos _asbp_instance_2 true)
              (Variables|/Game/ThirdPerson/Blueprints/BP_Instance.BP_Instance_C|SetPos _asbp_instance_2 _returnvalue_3)
              (goto _label))
            (else
              (goto _label))))
        (elif (Variables|Default|GetCloseBack)
          (Rendering|SetVisibility _cube1 true false)
          (Collision|SetCollisionProfileName _cube1 "BlockAll" true :!class /Script/Engine.PrimitiveComponent)
          (Variables|/Game/BP/BP_SliceCreator.BP_SliceCreator_C|SetWork (Variables|/Game/Variant_Combat/Blueprints/AI/BP_CombatEnemy.BP_CombatEnemy_C|GetSliceCreator (Variables|Default|GetEnemy)) true))))))

(event EventBeginPlay
  (bind _asbp_instance (Utilities|Casting|CastToBP_Instance (Game|GetGameInstance)))
  (Utilities|FlowControl|Sequence
    (:then_0
      (if (Variables|/Game/ThirdPerson/Blueprints/BP_Instance.BP_Instance_C|GetCanGrap _asbp_instance)
        (if (Utilities|Enum|Equal(Enum) (Variables|Default|GetLevelName) "Lvl_ThirdPerson")
          (Actor|DestroyActor))))
    (:then_1
      (if (Variables|/Game/ThirdPerson/Blueprints/BP_Instance.BP_Instance_C|GetCanSlice _asbp_instance)
        (if (Utilities|Enum|Equal(Enum) (Variables|Default|GetLevelName) "Lv2")
          (Actor|DestroyActor))))))

(event Collision|EventActorBeginOverlap
  (params (OtherActor :type Actor%20Object%20Reference)))

(event EventTick
  (params (DeltaSeconds :type Float%20%28single-precision%29)))

(fn ConstructionScript)

(fn Reset)