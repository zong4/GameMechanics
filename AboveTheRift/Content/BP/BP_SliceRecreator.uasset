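; BP_SliceRecreator restores a set of BP_Slice and BP_SliceCone actors to their original placement.
; On BeginPlay it records the transforms of the actors referenced in its Slices and SliceCones arrays.
; Reset destroys any still-valid actors in both arrays, clears them, then spawns fresh copies at the saved transforms and refills the arrays.
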(event EventBeginPlay
  (for _array_element (Variables|Default|GetSlices)
    (Utilities|Array|Add (Variables|Default|GetSliceTrans) (Transformation|GetActorTransform _array_element)))
  (for _array_element_2 (Variables|Default|GetSliceCones)
    (Utilities|Array|Add (Variables|Default|GetSliceConeTrans) (Transformation|GetActorTransform _array_element_2))))

(event Collision|EventActorBeginOverlap
  (params (OtherActor :type Actor%20Object%20Reference)))

(event EventTick
  (params (DeltaSeconds :type Float%20%28single-precision%29)))

(fn ConstructionScript)

(fn Reset
  (bind _slices (Variables|Default|GetSlices))
  (bind _slicecones (Variables|Default|GetSliceCones))
  (for _array_element _slices
    (Utilities|IsValid _array_element
      (:Is%20Valid
        (Actor|DestroyActor _array_element))))
  (Utilities|Array|Clear _slices)
  (for _array_element_2 _slicecones
    (Utilities|IsValid _array_element_2
      (:Is%20Valid
        (Actor|DestroyActor _array_element_2))))
  (Utilities|Array|Clear _slicecones)
  (for _array_element_3 (Variables|Default|GetSliceTrans)
    (bind _returnvalue (Game|SpawnActorfromClass "/Game/BP/BP_Slice.BP_Slice_C" _array_element_3 "Undefined" "MultiplyWithRoot" 0 0))
    (Utilities|Array|Add (Variables|Default|GetSlices) _returnvalue))
  (for _array_element_4 (Variables|Default|GetSliceConeTrans)
    (bind _returnvalue_2 (Game|SpawnActorfromClass "/Game/BP/BP_SliceCone.BP_SliceCone_C" _array_element_4 "Undefined" "MultiplyWithRoot" 0 0))
    (Utilities|Array|Add (Variables|Default|GetSliceCones) _returnvalue_2)))