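; BP_SliceCreator is a timed spawner that launches randomly chosen BP_Slice projectiles that can hit the player.
; On Tick, while Work is on, it spawns an actor from the Actors list each interval, setting its lifespan and zero linear damping.
; Velocity points at the player when TracePlayer and EnemyAttack are set, or along the right vector when TracePlayer is off.
; Its static mesh is hidden at BeginPlay.
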(event EventBeginPlay
  (Rendering|SetVisibility (Variables|Default|GetStaticMesh) false false))

(event Collision|EventActorBeginOverlap
  (params (OtherActor :type Actor%20Object%20Reference)))

(event EventTick
  (params (DeltaSeconds :type Float%20%28single-precision%29))
  (Variables|Default|SetSpawnTimer (+ (Variables|Default|GetSpawnTimer) DeltaSeconds))
  (if (> (Variables|Default|GetSpawnTimer) (Variables|Default|GetSpawnInv))
    (if (Variables|Default|GetWork)
      (Variables|Default|SetSpawnTimer 0.0)
      (bind _returnvalue (Game|SpawnActorfromClass (.OutItem (Utilities|Array|Random (Variables|Default|GetActors))) (Transformation|GetActorTransform) "Undefined" "MultiplyWithRoot" 0 0))
      (bind _asbp_slice (Utilities|Casting|CastToBP_Slice _returnvalue))
      (Actor|SetLifeSpan _asbp_slice (Variables|Default|GetLifeTime))
      (Variables|/Game/BP/BP_Slice.BP_Slice_C|SetCanHitPlayer _asbp_slice true)
      (Class|PrimitiveComponent|SetLinearDamping (Variables|/Game/BP/BP_Slice.BP_Slice_C|GetProceduralMesh _asbp_slice) 0.0)
      (if (Variables|Default|GetTracePlayer)
        (if (Variables|Default|GetEnemyAttack)
          (Physics|SetPhysicsLinearVelocity (Variables|/Game/BP/BP_Slice.BP_Slice_C|GetProceduralMesh _asbp_slice) (* (Math|Vector|Normalize (- (Transformation|GetActorLocation (Game|Player|GetPlayerPawn 0)) (Transformation|GetActorLocation))) (Variables|Default|GetForce)) false "None"))
        (else
          (Physics|SetPhysicsLinearVelocity (Variables|/Game/BP/BP_Slice.BP_Slice_C|GetProceduralMesh _asbp_slice) (* (Transformation|GetActorRightVector) (Variables|Default|GetForce)) false "None"))))))

(fn ConstructionScript)