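; BP_Slice is a sliceable physics actor whose impacts can knock back the player or hit combat enemies.
; Construction copies its static mesh into a procedural mesh, which Slice cuts along a plane with a lava-capped face, pushing the halves apart by opposing impulses.
; Hard hits release the player's rope and launch them, while non-player hits trigger enemy OnHit, each gated by flags and destroying the actor.
; Reset respawns it at its starting transform when allowed.
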(event OnComponentHit(ProceduralMesh)
  (params (HitComponent :type Primitive%20Component%20Object%20Reference) (OtherActor :type Actor%20Object%20Reference) (OtherComp :type Primitive%20Component%20Object%20Reference) (NormalImpulse :type Vector :default "0, 0, 0") (Hit :type Hit%20Result%20Structure%20%28by%20ref%29))
  (CallFunction|OnHit OtherActor NormalImpulse))

(event EventBeginPlay
  (Variables|Default|SetSpawn%20Transform (Transformation|GetActorTransform)))

(event Collision|EventActorBeginOverlap
  (params (OtherActor :type Actor%20Object%20Reference)))

(event EventTick
  (params (DeltaSeconds :type Float%20%28single-precision%29)))

(fn ConstructionScript
  (Class|KismetProceduralMeshLibrary|CopyProceduralMeshfromStaticMeshComponent (Variables|Debug|GetStaticMeshComponent) 0 (Variables|Default|GetProceduralMesh) true))

(fn Slice
  (params (PlanePosition :type Vector) (PlaneNormal :type Vector) (InProcMesh :type Procedural%20Mesh%20Component%20Object%20Reference) (B :type Float%20%28single-precision%29))
  (bind _returnvalue (* PlaneNormal B))
  (bind _outotherhalfprocmesh (Class|KismetProceduralMeshLibrary|SliceProceduralMesh InProcMesh PlanePosition PlaneNormal true "CreateNewSectionForCap" "/Game/Variant_Combat/Materials/M_Lava.M_Lava"))
  (Physics|SetSimulatePhysics _outotherhalfprocmesh true)
  (Variables|/Script/Engine.ActorComponent|SetComponentTags _outotherhalfprocmesh (Variables|/Script/Engine.ActorComponent|GetComponentTags (Variables|Default|GetProceduralMesh)))
  (Physics|AddImpulse InProcMesh _returnvalue "None" false)
  (Physics|AddImpulse _outotherhalfprocmesh (* _returnvalue -1.0) "None" false)
  (Collision|BindEventtoOnComponentHit _outotherhalfprocmesh (EventDispatchers|CreateEvent :!event BPSliceAutoGenFunc)))

(fn Reset
  (if (Variables|Default|GetCanReset)
    (Actor|DestroyActor)
    (bind _returnvalue (Game|SpawnActorfromClass "BP_Slice_C" (Variables|Default|GetSpawn%20Transform) "Undefined" "MultiplyWithRoot" 0 0))
    (Variables|BP_Slice_C|SetCanReset _returnvalue true)))

(fn OnHit
  (params (目标 :type Actor%20Object%20Reference) (LaunchVelocity :type Vector))
  (bind _returnvalue (* LaunchVelocity 0.005))
  (bind (_x _y _z) (Math|Vector|BreakVector _returnvalue))
  (if (Actor|ActorHasTag 目标 "Player")
    (if (Variables|Default|GetCanHitPlayer)
      (if (> (Math|Vector|VectorLength LaunchVelocity) 1e+04)
        (bind _asbp_third_person_character (Utilities|Casting|CastToBP_ThirdPersonCharacter 目标))
        (Default|ReleaseRope _asbp_third_person_character)
        (Character|LaunchCharacter _asbp_third_person_character (Math|Vector|MakeVector _x _y _z) true true)
        (Actor|DestroyActor)))
    (elif true
      (if (Variables|Default|GetCanHitEnemy)
        (bind _asbp_combat_enemy (Utilities|Casting|CastToBP_CombatEnemy 目标))
        (Default|OnHit _asbp_combat_enemy)
        (Actor|DestroyActor)))))

(fn BPSliceAutoGenFunc
  (params (HitComponent :type Primitive%20Component%20Object%20Reference) (OtherActor :type Actor%20Object%20Reference) (OtherComp :type Primitive%20Component%20Object%20Reference) (NormalImpulse :type Vector) (Hit :type Hit%20Result%20Structure%20%28by%20ref%29))
  (bind _returnvalue (* NormalImpulse 0.005))
  (bind (_x _y) (Math|Vector|BreakVector _returnvalue))
  (if (Actor|ActorHasTag OtherActor "Player")
    (if (> (Math|Vector|VectorLength "0, 0, 0") 1e+04)
      (if (Variables|Default|GetCanHitPlayer)
        (bind _asbp_third_person_character (Utilities|Casting|CastToBP_ThirdPersonCharacter OtherActor))
        (Character|LaunchCharacter _asbp_third_person_character (Math|Vector|MakeVector _x _y 0.0) true true)
        (Actor|DestroyActor)
        (return)))
    (elif true
      (if (Variables|Default|GetCanHitEnemy)
        (bind _asbp_combat_enemy (Utilities|Casting|CastToBP_CombatEnemy OtherActor))
        (Default|OnHit _asbp_combat_enemy)
        (Actor|DestroyActor)))))