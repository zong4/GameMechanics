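; Actor Blueprint for a platform that keeps moving between randomly chosen positions.
; BeginPlay converts the Positions offsets to world space by adding the actor's starting location.
; When idle, Tick picks a random index differing from the last, and a timeline lerps the actor there, re-arming on finish.
; Every timeline update also notifies the navigation system that NavVolume's bounds changed, triggering a navmesh update as the platform moves.
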(event EventBeginPlay
  (for (_array_element _array_index) (Variables|Default|GetPositions)
    (Utilities|Array|SetArrayElem (Variables|Default|GetPositions) _array_index (+ _array_element (Transformation|GetActorLocation))))
  (for _array_element_2 (Variables|Default|GetPositions)
    _))

(event Collision|EventActorBeginOverlap
  (params (OtherActor :type Actor%20Object%20Reference)))

(event EventTick
  (params (DeltaSeconds :type Float%20%28single-precision%29))
  (bind _positions (Variables|Default|GetPositions))
  (if (Variables|Default|GetWaitMove)
    (if (> (Utilities|Array|Length _positions) 0)
      (bind _output_get (Variables|Default|SetIndex (.OutIndex (Utilities|Array|Random _positions))))
      (if (!= _output_get (Variables|Default|GetLastIndex))
        (Variables|Default|SetWaitMove false)
        (Variables|Default|SetLastIndex _output_get)
        (bind _output_get_2 (Variables|Default|SetStartPos (Transformation|GetActorLocation)))
        (bind _alpha (Timeline|时间轴 PlayFromStart)
          (:Update
            (Transformation|SetActorLocation (Math|Vector|Lerp(Vector) _output_get_2 (Utilities|Array|Get(acopy) (Variables|Default|GetPositions) (Variables|Default|GetIndex)) _alpha) false false)
            (Class|NavigationSystemV1|OnNavigationBoundsUpdated (Class|NavigationSystemV1|GetNavigationSystem) (Variables|Default|GetNav%20Volume)))
          (:Finished
            (Variables|Default|SetWaitMove true)))))))

(fn ConstructionScript)