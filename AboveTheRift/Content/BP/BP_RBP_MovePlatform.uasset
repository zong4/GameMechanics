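; Moving platform that travels through a list of waypoints in an endless cycle.
; BeginPlay converts the Positions offsets to world space around the start location and sets the timeline play rate from Speed.
; When WaitMove is set, Tick starts a timeline that lerps the actor to the current waypoint, then advances the index with wraparound.
; Record and DeltaPos expose displacement since the last recorded position.
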(event EventBeginPlay
  (for (_array_element _array_index) (Variables|Default|GetPositions)
    (Utilities|Array|SetArrayElem (Variables|Default|GetPositions) _array_index (+ _array_element (Transformation|GetActorLocation))))
  (for _array_element_2 (Variables|Default|GetPositions)
    _)
  (Components|Timeline|SetPlayRate (Variables|Default|Get时间轴) (Variables|Default|GetSpeed)))

(event Collision|EventActorBeginOverlap
  (params (OtherActor :type Actor%20Object%20Reference)))

(event EventTick
  (params (DeltaSeconds :type Float%20%28single-precision%29))
  (if (Variables|Default|GetWaitMove)
    (if (> (Utilities|Array|Length (Variables|Default|GetPositions)) 0)
      (Variables|Default|SetWaitMove false)
      (bind _output_get (Variables|Default|SetStartPos (Transformation|GetActorLocation)))
      (bind _alpha (Timeline|时间轴 PlayFromStart)
        (:Update
          (Transformation|SetActorLocation (Math|Vector|Lerp(Vector) _output_get (Utilities|Array|Get(acopy) (Variables|Default|GetPositions) (Variables|Default|GetIndex)) _alpha) false false))
        (:Finished
          (Variables|Default|SetIndex (Math|Integer|%(Integer) (+ (Variables|Default|GetIndex) 1) (Utilities|Array|Length (Variables|Default|GetPositions))))
          (Variables|Default|SetWaitMove true))))))

(fn ConstructionScript)

(fn DeltaPos
  (return (- (Transformation|GetActorLocation) (Variables|Default|GetRecordPos))))

(fn Record
  (Variables|Default|SetRecordPos (Transformation|GetActorLocation)))