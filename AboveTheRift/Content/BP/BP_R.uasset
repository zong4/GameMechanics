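; BP_R is an actor that shows the BP_HintR hint widget when its cone count reaches zero.
; Tick polls the Reset function, which only checks whether ConeCnt is zero and changes no state.
; The Reseted flag makes the hint fire once, adding the widget to the viewport and removing it after a short delay.
; Nothing in this graph updates ConeCnt or clears the flag.
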(event EventBeginPlay)

(event Collision|EventActorBeginOverlap
  (params (OtherActor :type Actor%20Object%20Reference)))

(event EventTick
  (params (DeltaSeconds :type Float%20%28single-precision%29))
  (bind _res (CallFunction|Reset))
  (if _res
    (if (not (Variables|Default|GetReseted))
      (Variables|Default|SetReseted true)
      (bind _returnvalue (UserInterface|CreateWidget "/Game/BP/BP_HintR.BP_HintR_C"))
      (UserInterface|Viewport|AddtoViewport _returnvalue 0)
      (Utilities|FlowControl|Delay 1.5)
      (Widget|RemovefromParent _returnvalue))))

(fn ConstructionScript)

(fn Reset
  (if (== (Variables|Default|GetConeCnt) 0)
    (return true)
    (else
      (return false))))